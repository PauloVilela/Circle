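; MultyCollorManiger is a puzzle manager that opens doors when a four-part puzzle is solved.
; Its PuzzelIsDone event checks the flags P1 through P4 in nested branches and, only when all are true, calls OpenDoor on every entry in the Door array.
; The graph only reads the flags and does not set them or call the event itself.
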(event `PuzzelIsDone`
  (if (`self.P1`)
    (if (`self.P2`)
      (if (`self.P3`)
        (if (`self.P4`)
          (for _array_element (`self.Door`)
            (`/Game/Blueprints/Acters/Door_BP.OpenDoor` _array_element)))))))

(fn `UserConstructionScript`)