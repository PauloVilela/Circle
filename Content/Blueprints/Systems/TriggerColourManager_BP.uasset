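; TriggerColourManager_BP is a manager that opens two doors through a timed colour-matching trigger, with only Cyan handled.
; RemoveColour with Cyan starts a ten-second window, which Tick counts down through a one-second Delay and prints.
; While the window is open, AddColour stores a differing colour as current, or opens both doors when the incoming colour matches a current Cyan.
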(event `self.ReceiveTick`
  (params (DeltaSeconds :type "Float (single-precision)"))
  ;[1 1 1] Timer
  (if (> (`self.Timer`) 0)
    (`KismetSystemLibrary.Delay` 1.0)
    (bind _output_get (set `self.Timer` (- (`self.Timer`) 1)))
    (`KismetSystemLibrary.PrintString` (`KismetStringLibrary.Conv_IntToString` _output_get))))

(event `Add Colour`
  (params (Colour :type "/Game/Blueprints/Acters/Colour_Enum Enum" :default "NewEnumerator0"))
  (if (> (`self.Timer`) 0)
    (if (== Colour (`self.CurrentColour`))
      (switch `/Game/Blueprints/Acters/Colour_Enum` (`self.CurrentColour`)
        (:`NewEnumerator0`
          (`/Game/Blueprints/Acters/Door_BP.OpenDoor` (`self.Door`))
          (`/Game/Blueprints/Acters/Door_BP.OpenDoor` (`self.Door2`))))
      (else
        (set `self.CurrentColour` Colour)))))

(event `RemoveColour`
  (params (Colour :type "/Game/Blueprints/Acters/Colour_Enum Enum" :default "NewEnumerator0"))
  (switch `/Game/Blueprints/Acters/Colour_Enum` Colour
    (:`NewEnumerator0`
      (set `self.Timer` 10))))

(fn `UserConstructionScript`)