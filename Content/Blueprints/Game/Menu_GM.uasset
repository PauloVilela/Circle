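; Game mode for the start menu that sets up local players and shows the menu widget.
; On BeginPlay it creates players by index up to NumberOfPlayers, stores their controllers in an array, then adds a StartMenu_WBP widget to the viewport.
; A RemovePlayers event loops over the stored controllers and removes each player, destroying its pawn.
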(event `self.ReceiveBeginPlay`
  ;[1 1 1] Addplayers to menu
  (for _index (range (+ (`self.NumberOfPlayers`) 1))
    (bind _returnvalue (`GameplayStatics.CreatePlayer` _index))
    (`KismetArrayLibrary.Array_Add` (`self.MenuCpontrollers_BP`) _returnvalue))
  (bind _returnvalue_2 (`|CreateWidget` "/Game/Blueprints/UI/StartMenu_WBP.StartMenu_WBP_C"))
  (bind _output_get (set `self.StartMenu_WBP` _returnvalue_2))
  (`UserWidget.AddToViewport` _output_get 0))

(event `RemovePlayers`
  ;[1 1 1] Remove players
  (for _array_element (`self.MenuCpontrollers_BP`)
    (`GameplayStatics.RemovePlayer` _array_element true)))

(fn `UserConstructionScript`)