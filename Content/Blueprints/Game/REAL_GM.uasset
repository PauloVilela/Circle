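; REAL_GM sets up local multiplayer on BeginPlay, giving each player a controller, a character and a HUD.
; It collects the level's PlayerStarts, then creates the local players in one loop driven by NumberOfPlayers.
; A second loop spawns each PlayersArray class at the same-index start, possesses it and adds a per-player HUD widget.
; Every spawn takes the first loop's CreatePlayer output as Owner, rather than looking up its own controller.
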(event `self.ReceiveBeginPlay`
  (bind _numberofplayers (`self.NumberOfPlayers`))
  (bind _outactors (`GameplayStatics.GetAllActorsOfClass` "/Script/Engine.PlayerStart"))
  (set `self.SpawnPoints` _outactors)
  (for _index (range (+ _numberofplayers 1))
    ;[1 1 1] Create Controller
    (bind _returnvalue (`GameplayStatics.CreatePlayer` _index)))
  ;[1 1 1] SpawnCharacters
  (for _index_2 (range (+ _numberofplayers 1))
    (bind _returnvalue_2 (`|SpawnActorFromClass` (`|GetArrayItem` (`self.PlayersArray`) _index_2) (`self.GetTransform` (`|GetArrayItem` (`self.SpawnPoints`) _index_2)) "Undefined" "OverrideRootScale" _returnvalue null))
    (bind _returnvalue_3 (`GameplayStatics.GetPlayerController` _index_2))
    (`Controller.Possess` _returnvalue_3 _returnvalue_2)
    (bind _returnvalue_4 (`|CreateWidget` "/Game/Blueprints/UI/HUD_Widget.HUD_Widget_C" _returnvalue_3))
    (`UserWidget.AddToPlayerScreen` _returnvalue_4 0)))

(fn `UserConstructionScript`)