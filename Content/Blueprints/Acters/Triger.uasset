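; Trigger actor that opens a pair of doors while something overlaps its box volume.
; Box begin overlap casts the Door1 and Door2 references to Door and calls OpenDoor on each, and end overlap calls CloseDoor the same way.
; The overlapping actor is never filtered or counted, and a failed cast on Door1 also skips Door2.
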(event `self.Box.OnComponentBeginOverlap`
  (params (OverlappedComponent :type "PrimitiveComponent Object Reference") (OtherActor :type "Actor Object Reference") (OtherComp :type "PrimitiveComponent Object Reference") (OtherBodyIndex :type Integer) (bFromSweep :type Boolean) (SweepResult :type "HitResult Structure (by ref)"))
  (bind _asdoor (cast `/Game/Blueprints/Acters/Door` (`self.Door 1`)))
  (`/Game/Blueprints/Acters/Door.OpenDoor` _asdoor)
  (bind _asdoor_2 (cast `/Game/Blueprints/Acters/Door` (`self.Door 2`)))
  (`/Game/Blueprints/Acters/Door.OpenDoor` _asdoor_2))

(event `self.Box.OnComponentEndOverlap`
  (params (OverlappedComponent :type "PrimitiveComponent Object Reference") (OtherActor :type "Actor Object Reference") (OtherComp :type "PrimitiveComponent Object Reference") (OtherBodyIndex :type Integer))
  (bind _asdoor (cast `/Game/Blueprints/Acters/Door` (`self.Door 1`)))
  (`/Game/Blueprints/Acters/Door.CloseDoor` _asdoor)
  (bind _asdoor_2 (cast `/Game/Blueprints/Acters/Door` (`self.Door 2`)))
  (`/Game/Blueprints/Acters/Door.CloseDoor` _asdoor_2))

(fn `UserConstructionScript`)