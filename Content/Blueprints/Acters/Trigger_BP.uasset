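; Trigger actor that opens one or two linked Door_BP doors when its trigger is overlapped and a line trace registers a hit.
; While overlapped, Tick traces on the Camera channel between the TraceStart and TraceEnd components until it hits, then a DoOnce opens the doors.
; Ending the overlap clears the hit state, closes the doors and resets the DoOnce.
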(event `self.ReceiveTick`
  (params (DeltaSeconds :type "Float (single-precision)"))
  ;[1 1 1] On Trigger Test
  (if (`self.Overlap?`)
    (if (not (`self.RaycastHit?`))
      (bind (_outhit _returnvalue) (`KismetSystemLibrary.LineTraceSingle` :`Start` (`SceneComponent.K2_GetComponentLocation` (`self.TraceStart`)) :`End` (`SceneComponent.K2_GetComponentLocation` (`self.TraceEnd`)) :`TraceChannel` "TraceTypeQuery2" :`TraceColor` (struct :`R` 1.0 :`G` 0.88979 :`A` 1.0) :`TraceHitColor` (struct :`R` 1.0 :`B` 0.052632 :`A` 1.0)))
      (bind _output_get (set `self.RaycastHit?` _returnvalue))
      (if _output_get
        (`KismetSystemLibrary.PrintString` (`KismetStringLibrary.Conv_BoolToString` _output_get))
        (`/Engine/EditorBlueprintResources/StandardMacros.DoOnce` false :!label _label
          (:`Completed`
            (bind _asdoor_bp (cast `/Game/Blueprints/Acters/Door_BP` (`self.Door 1`)))
            (`/Game/Blueprints/Acters/Door_BP.OpenDoor` _asdoor_bp)
            (if (`self.2Doors`)
              (bind _asdoor_bp_2 (cast `/Game/Blueprints/Acters/Door_BP` (`self.Door 2`)))
              (`/Game/Blueprints/Acters/Door_BP.OpenDoor` _asdoor_bp_2))))))))

(event `ResetDoOnce`
  ;[1 1 1] On Trigger Test
  (goto _label :!via `Reset`))

(event `self.Trigger.OnComponentBeginOverlap`
  (params (OverlappedComponent :type "PrimitiveComponent Object Reference") (OtherActor :type "Actor Object Reference") (OtherComp :type "PrimitiveComponent Object Reference") (OtherBodyIndex :type Integer) (bFromSweep :type Boolean) (SweepResult :type "HitResult Structure (by ref)"))
  ;[1 1 1] On Trigger Test
  (set `self.Overlap?` true))

(event `self.Trigger.OnComponentEndOverlap`
  (params (OverlappedComponent :type "PrimitiveComponent Object Reference") (OtherActor :type "Actor Object Reference") (OtherComp :type "PrimitiveComponent Object Reference") (OtherBodyIndex :type Integer))
  ;[1 1 1] On Trigger Test
  (set `self.Overlap?` false)
  (bind _output_get (set `self.RaycastHit?` false))
  (if (not _output_get)
    (bind _asdoor_bp (cast `/Game/Blueprints/Acters/Door_BP` (`self.Door 1`)))
    (`/Game/Blueprints/Acters/Door_BP.CloseDoor` _asdoor_bp)
    (`self.ResetDoOnce`)
    (if (`self.2Doors`)
      (bind _asdoor_bp_2 (cast `/Game/Blueprints/Acters/Door_BP` (`self.Door 2`)))
      (`/Game/Blueprints/Acters/Door_BP.CloseDoor` _asdoor_bp_2))))

(fn `UserConstructionScript`)